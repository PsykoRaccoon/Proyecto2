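; BP_WaveGameMode is a game mode that runs enemy waves separated by five-second interludes.
; Each wave loads its class-count enemy pool from DT_WaveData by wave number; the AlgorithmicWave fallback is empty.
; Random picks from the pool queue on random BP_EnemySpawners up to EnemyLimit, refilling as enemies die.
; Killing all enemies or exhausting the countdown ends the wave, clearing spawners, with dispatchers reporting progress.
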(event Custom|StartTimer
  ;[0.15 0.15 0.15 0.5] WaveTimer
  (if (== (Variables|Default|GetSeconds) 0)
    (if (== (Variables|Default|GetMinutes) 0)
      (Utilities|FlowControl|DoOnce false
        (:Completed
          (if (not (Variables|Default|GetOnBreak))
            (CallFunction|Interlude)
            (else
              (Variables|Default|SetOnBreak false)))))
      (else
        (Variables|Default|SetSeconds 59)
        (Variables|Default|SetMinutes (- (Variables|Default|GetMinutes) 1))
        (Default|CallOnTimerUpdated (Variables|Default|GetMinutes) (Variables|Default|GetSeconds) :!label _label)))
    (else
      (Variables|Default|SetSeconds (- (Variables|Default|GetSeconds) 1))
      (goto _label))))

(event Custom|BeginNextWave
  (CallFunction|StartWave))

(event Custom|Interlude
  (bind _returnvalue (Utilities|Time|SetTimerbyEvent (delegate Custom|BeginNextWave) 5.0))
  (Variables|Default|SetInterludeTimer _returnvalue)
  (CallFunction|EndWave))

(event Custom|ResetTimer
  ;[0.15 0.15 0.15 0.5] WaveTimer
  (Utilities|FlowControl|DoOnce false) ; enters at Reset
)

(event EventBeginPlay
  (CallFunction|Interlude))

(event EventTick
  (params (DeltaSeconds :type Float%20%28single-precision%29)))

(fn ConstructionScript)

(fn OnEnemyEliminated
  (Math|Integer|DecrementInt (Variables|Default|GetEnemiesRemaining)
    (:%20%20
      (bind _result (Math|Integer|IncrementInt (Variables|Default|GetEnemiesKilled))
        (:%20%20
          (Default|CallOnEnemyKilled _result (Variables|Default|GetTotalEnemies) (Variables|Default|GetScoreCollected))
          (if (< (Variables|Default|GetEnemiesRemaining) (Variables|Default|GetEnemyLimit))
            (if (== (Variables|Default|GetEnemiesRemaining) 0)
              (CallFunction|Interlude)
              (Variables|Default|SetOnBreak true))
            (else
              (CallFunction|AddEnemytoQueue))))))))

(fn AddEnemytoQueue
  (Default|AddEnemytoQueue (.OutItem (Utilities|Array|Random (Variables|Default|GetEnemySpawners))) (CallFunction|GetEnemyfromPool)))

(fn GetEnemiesSpawners
  (bind _outactors (Actor|GetAllActorsOfClass "/Game/WaveSpawnSystem/EnemySpawners/BP_EnemySpawner.BP_EnemySpawner_C"))
  (Variables|Default|SetEnemySpawners _outactors))

(fn GetEnemyfromPool
  (bind _keys (Utilities|Map|Keys (Variables|Default|GetEnemyPool)))
  (bind _output_get (LocalVariables|SetLocalEnemy_Class (.OutItem (Utilities|Array|Random _keys))))
  (if (<= (- (.Value (Utilities|Map|Find (Variables|Default|GetEnemyPool) _output_get)) 1) 0)
    (Utilities|Map|Remove (Variables|Default|GetEnemyPool) (LocalVariables|GetLocalEnemy_Class))
    (else
      (Utilities|Map|Add (Variables|Default|GetEnemyPool) (LocalVariables|GetLocalEnemy_Class) (- (.Value (Utilities|Map|Find (Variables|Default|GetEnemyPool) _output_get)) 1))))
  (return (LocalVariables|GetLocalEnemy_Class)))

(fn StartWave
  (Math|Integer|IncrementInt (Variables|Default|GetWaveNumber)
    (:%20%20
      (CallFunction|GetEnemiesSpawners)
      (CallFunction|WaveClock)
      (CallFunction|BuildWave)
      (Default|CallOnstackWave (Variables|Default|GetWaveNumber) (Variables|Default|GetEnemiesKilled) (Variables|Default|GetTotalEnemies) (Variables|Default|GetScoreCollected))
      (CallFunction|ResetTimer))))

(fn EndWave
  (Variables|Default|SetEnemiesKilled 0)
  (Variables|Default|SetMinutes 0)
  (Variables|Default|SetSeconds 0)
  (for _array_element (Variables|Default|GetEnemySpawners)
    (Default|ClearAllEnemies _array_element))
  (Default|CallOnWaveEnd))

(fn GetPoolSize
  (bind _values (Utilities|Map|Values (Variables|Default|GetEnemyPool)))
  (for _array_element _values
    (LocalVariables|SetLocal_EnemyPool (+ _array_element (LocalVariables|GetLocal_EnemyPool))))
  (return (LocalVariables|GetLocal_EnemyPool)))

(fn BuildEnemyPool
  (bind _enemypoolsize (CallFunction|GetPoolSize))
  (bind _returnvalue (Utilities|GetDataTableRow "/Game/WaveSpawnSystem/WaveData/DT_WaveData.DT_WaveData" (Utilities|String|StringToName (Utilities|String|ToString(Integer) (Variables|Default|GetWaveNumber))))
    (:then
      (Variables|Default|SetEnemyPool (Utilities|Struct|BreakS_WaveInfo _returnvalue))
      (Variables|Default|SetEnemiesRemaining _enemypoolsize)
      (Variables|Default|SetTotalEnemies _enemypoolsize))
    (:RowNotFound
      (CallFunction|AlgorithmicWave))))

(fn AlgorithmicWave)

(fn BuildWave
  (CallFunction|BuildEnemyPool)
  (for _index (range 0 (- (Math|Integer|Min(Integer) (CallFunction|GetPoolSize) (Variables|Default|GetEnemyLimit)) 1))
    (CallFunction|AddEnemytoQueue)))

(fn CountDownTimer
  (Utilities|Time|SetTimerbyEvent (EventDispatchers|CreateEvent :!event Custom|StartTimer) 1.0 true)
  (return (Variables|Default|GetMinutes) (Variables|Default|GetSeconds)))

(fn WaveClock
  (bind _output_get (Variables|Default|SetStoredSeconds (+ (Variables|Default|GetStoredSeconds) 20)))
  (if (>= _output_get 0)
    (Variables|Default|SetStoredSeconds 0)
    (bind _result (Math|Integer|IncrementInt (Variables|Default|GetStoredMinutes))
      (:%20%20
        (Variables|Default|SetMinutes _result)))
    (else
      ;[0.15 0.15 0.15 0.5] Si no funciona algo, checar esto
      (Variables|Default|SetSeconds (Variables|Default|GetSeconds))
      (Variables|Default|SetMinutes (Variables|Default|GetStoredMinutes)))))